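; Steam game instance Blueprint that hosts and joins multiplayer sessions through Advanced Sessions nodes.
; Create_Session creates a session and, on success, opens ThirdPersonExampleMap as a listen server.
; Join_Session searches all server types, runs an empty loop over the results, then joins using the loop's final element.
; Join success or failure only prints a debug string.
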(event `Create_Session`
  (`CreateSessionCallbackProxyAdvanced.CreateAdvancedSession` :`PlayerController` (`GameplayStatics.GetPlayerController` 0)
    (:`OnSuccess`
      (`GameplayStatics.OpenLevel` "ThirdPersonExampleMap" true "listen"))))

(event `Join_Session`
  (bind _results (`FindSessionsCallbackProxyAdvanced.FindSessionsAdvanced` (`GameplayStatics.GetPlayerController` 0) 10 false "AllServers")
    (:`OnSuccess`
      (bind _output_get (set `self.FoundSessions` _results))
      (for _array_element _output_get
        _)
      (`JoinSessionCallbackProxy.JoinSession` (`GameplayStatics.GetPlayerController` 0) _array_element
        (:`OnSuccess`
          (`KismetSystemLibrary.PrintString` "Funciono"))
        (:`OnFailure`
          (`KismetSystemLibrary.PrintString` "No Funciono"))))))